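; Spawner actor that builds a chain of BP_Tunnel segments along +X, populated with random health packs and enemies.
; SpawnTunnel randomizes each segment's wall and rotation speed, tints its material, links it to the spawner and registers its spawned pickup and enemies.
; SpawnTunnelAtSpawnPoint extends the chain from the newest segment, with EnemyEV scaling enemy spawn attempts.
; On BeginPlay, SpawnInitialTunnels clears existing tunnels and lays an enemy-free starting run.
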(event `self.ReceiveBeginPlay`
  (`self.SpawnTunnel` (0.0 0.0 0.0))
  (`self.SpawnInitialTunnels`))

(fn `SpawnInitialTunnels`
  (`|ExecutionSequence`
    (:`then_0`
      (bind _outactors (`GameplayStatics.GetAllActorsOfClass` "/Game/InfiniteMatrix/Blueprints/BP_Tunnel.BP_Tunnel_C"))
      (for _array_element _outactors
        (`self.K2_DestroyActor` _array_element)))
    (:`then_1`
      (for _ (range 4)
        (`/Engine/EditorBlueprintResources/StandardMacros.IsValid` (`self.NewestTunnel`)
          (:`Is Valid`
            (`self.SpawnTunnelAtSpawnPoint` 0.0))
          (:`Is Not Valid`
            (`self.SpawnTunnel` (`self.K2_GetActorLocation` (`GameplayStatics.GetPlayerPawn` 0)) 0.0)))))))

(fn `SpawnTunnel`
  (params (SpawnLocation :type "Vector Structure") (EnemyEV :type "Float (double-precision)" :default 2.0))
  (bind _returnvalue (`|SpawnActorFromClass` "/Game/InfiniteMatrix/Blueprints/BP_Tunnel.BP_Tunnel_C" (`KismetMathLibrary.MakeTransform` SpawnLocation) "Undefined" "OverrideRootScale" null null))
  (bind _output_get (set `self.NewestTunnel` _returnvalue))
  (set `/Game/InfiniteMatrix/Blueprints/BP_Tunnel.TunnelSpawner` self _output_get)
  (`/Game/InfiniteMatrix/Blueprints/BP_Tunnel.RandomizeWall` _output_get)
  (set `/Game/InfiniteMatrix/Blueprints/BP_Tunnel.RotationSpeed` (`KismetMathLibrary.RandomFloatInRange` 20.0 65.0) _output_get)
  (bind _returnvalue_2 (`PrimitiveComponent.CreateDynamicMaterialInstance` (`StaticMeshActor.StaticMeshComponent` _output_get) 0 null "None"))
  (`MaterialInstanceDynamic.SetVectorParameterValue` _returnvalue_2 "TextColor" (`self.TunnelColor`))
  (if (`KismetMathLibrary.RandomBoolWithWeight` (`self.HealthPackRarity`))
    (bind _returnvalue_3 (`|SpawnActorFromClass` "/Game/InfiniteMatrix/Blueprints/HealthPack.HealthPack_C" (`KismetMathLibrary.MakeTransform` (+ SpawnLocation (`KismetMathLibrary.MakeVector` (`KismetMathLibrary.RandomFloatInRange` 550.0 2000.0) (`KismetMathLibrary.RandomFloatInRange` -150.0 150.0) (`KismetMathLibrary.RandomFloatInRange` -150.0 150.0)))) "Undefined" "OverrideRootScale" null null))
    (set `/Game/InfiniteMatrix/Blueprints/BP_Tunnel.Pack` _returnvalue_3 _output_get))
  (for _ (range 1 (+ (* (`KismetMathLibrary.FTrunc` EnemyEV) 2) 1))
    (if (`KismetMathLibrary.RandomBoolWithWeight` (`self.EnemyRarity`))
      (bind _returnvalue_4 (`|SpawnActorFromClass` "/Game/InfiniteMatrix/Blueprints/Enemy.Enemy_C" (`KismetMathLibrary.MakeTransform` (+ SpawnLocation (`KismetMathLibrary.MakeVector` (`KismetMathLibrary.RandomFloatInRange` 1000.0 2000.0) (`KismetMathLibrary.RandomFloatInRange` -150.0 150.0) (`KismetMathLibrary.RandomFloatInRange` -150.0 150.0)))) "Undefined" "OverrideRootScale" null null))
      (`KismetArrayLibrary.Array_Add` (`/Game/InfiniteMatrix/Blueprints/BP_Tunnel.EnemyArr` _output_get) _returnvalue_4))))

(fn `SpawnTunnelAtSpawnPoint`
  (params (EnemyEV :type "Float (double-precision)" :default 1.0))
  (`self.SpawnTunnel` (+ (`SceneComponent.K2_GetComponentLocation` (`Actor.RootComponent` (`self.NewestTunnel`))) (2500.0 0.0 0.0)) EnemyEV))

(fn `UserConstructionScript`)