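; Tunnel segment for an endless tunnel game, with a spinning holed wall whose mesh and roll RandomizeWall can randomize.
; Player overlap with the trigger has TunnelSpawner add a segment, destroys this one with its pack and enemies, and adds score.
; Wall hits cut health, then either trigger death or break the wall and deduct score.
; Health also tints all tunnels green-to-red through dynamic materials and updates the spawner's color.
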(event `self.ReceiveBeginPlay`)

(event `self.ReceiveTick`
  (params (DeltaSeconds :type "Float (single-precision)"))
  (bind _wallmesh (`self.WallMesh`))
  (`/Engine/EditorBlueprintResources/StandardMacros.IsValid` _wallmesh
    (:`Is Valid`
      (`SceneComponent.K2_AddLocalRotation` _wallmesh (`KismetMathLibrary.MakeRotator` (* DeltaSeconds (`self.RotationSpeed`))) false false))))

(event `self.TriggerZone.OnComponentBeginOverlap`
  (params (OverlappedComponent :type "PrimitiveComponent Object Reference") (OtherActor :type "Actor Object Reference") (OtherComp :type "PrimitiveComponent Object Reference") (OtherBodyIndex :type Integer) (bFromSweep :type Boolean) (SweepResult :type "HitResult Structure (by ref)"))
  (bind _pack (`self.Pack`))
  (bind _asbp_player (cast `/Game/InfiniteMatrix/Blueprints/BP_Player` OtherActor))
  (`/Game/InfiniteMatrix/Blueprints/BP_TunnelSpawner.SpawnTunnelAtSpawnPoint` (`self.TunnelSpawner`) 1.0)
  (`self.K2_DestroyActor`)
  (bind _output_get (set `/Game/InfiniteMatrix/Blueprints/BP_Player.Score` (+ (`/Game/InfiniteMatrix/Blueprints/BP_Player.Score` _asbp_player) 1) _asbp_player))
  (`/Game/InfiniteMatrix/Blueprints/WB_Score.UpdateScore` (`/Game/InfiniteMatrix/Blueprints/BP_Player.WB_Score` _asbp_player) _output_get)
  (`/Engine/EditorBlueprintResources/StandardMacros.IsValid` _pack
    (:`Is Valid`
      (`self.K2_DestroyActor` _pack)
      (for _array_element (`self.EnemyArr`)
        (`/Engine/EditorBlueprintResources/StandardMacros.IsValid` _array_element
          (:`Is Valid`
            (`self.K2_DestroyActor` _array_element)))))))

(event `self.WallMesh.OnComponentHit`
  (params (HitComponent :type "PrimitiveComponent Object Reference") (OtherActor :type "Actor Object Reference") (OtherComp :type "PrimitiveComponent Object Reference") (NormalImpulse :type "Vector Structure") (Hit :type "HitResult Structure (by ref)"))
  (bind _asbp_player (cast `/Game/InfiniteMatrix/Blueprints/BP_Player` OtherActor))
  (bind _output_get (set `/Game/InfiniteMatrix/Blueprints/BP_Player.Health` (- (`/Game/InfiniteMatrix/Blueprints/BP_Player.Health` _asbp_player) 20.0) _asbp_player))
  (`self.UpdateWallColorByHealthValue` _output_get)
  (`/Game/InfiniteMatrix/Blueprints/WB_HealthBar.UpdateHaelthBar` (`/Game/InfiniteMatrix/Blueprints/BP_Player.WB_HealthBar` _asbp_player) _output_get)
  (if (<= _output_get 0.0)
    (set `/Game/InfiniteMatrix/Blueprints/BP_Player.IsDead` true _asbp_player) ; death
    (`/Game/InfiniteMatrix/Blueprints/BP_Player.DisplayRestart` _asbp_player)
    (else
      (`ActorComponent.K2_DestroyComponent` HitComponent)
      (set `/Game/InfiniteMatrix/Blueprints/BP_Player.Score` (- (`/Game/InfiniteMatrix/Blueprints/BP_Player.Score` _asbp_player) 1) _asbp_player))))

(event `UpdateWallColorByHealthValue`
  (params (Health :type "Float (double-precision)"))
  (bind _returnvalue (/ Health 100.0))
  (bind _returnvalue_2 (- 1.0 _returnvalue))
  (bind _linearcolor (make `LinearColor` _returnvalue_2 _returnvalue (* _returnvalue_2 0.2)))
  (set `/Game/InfiniteMatrix/Blueprints/BP_TunnelSpawner.TunnelColor` _linearcolor (`self.TunnelSpawner`))
  (bind _outactors (`GameplayStatics.GetAllActorsOfClass` "BP_Tunnel_C"))
  (for _array_element _outactors
    (bind _returnvalue_3 (`PrimitiveComponent.CreateDynamicMaterialInstance` (`StaticMeshActor.StaticMeshComponent` _array_element) 0 null "None"))
    (`MaterialInstanceDynamic.SetVectorParameterValue` _returnvalue_3 "TextColor" _linearcolor)))

(fn `RandomizeWall`
  (`StaticMeshComponent.SetStaticMesh` (`self.WallMesh`) (select `int` (`KismetMathLibrary.RandomIntegerInRange` 0 3) :`0` "/Game/InfiniteMatrix/Meshes/SM_Hole_01.SM_Hole_01" :`1` "/Game/InfiniteMatrix/Meshes/SM_Hole_02.SM_Hole_02" :`2` "/Game/InfiniteMatrix/Meshes/SM_Hole_03.SM_Hole_03" :`3` "/Game/InfiniteMatrix/Meshes/SM_Hole_04.SM_Hole_04" :!type "StaticMesh Object Reference"))
  (`SceneComponent.K2_AddLocalRotation` (`self.WallMesh`) (`KismetMathLibrary.MakeRotator` (`KismetMathLibrary.RandomFloatInRange` 0.0 360.0)) false false))

(fn `UserConstructionScript`)