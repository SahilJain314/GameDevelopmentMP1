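; Enemy actor that damages the player when its Skull component hits BP_Player, then destroys itself.
; Each hit subtracts a fixed amount of health, updates the health bar widget and recolors the first BP_Tunnel's walls by health.
; The death check subtracts damage again from the already reduced health before showing restart and flagging the player dead.
; An unconnected score-increment chain never runs.
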(event `self.Skull.OnComponentHit`
  (params (HitComponent :type "PrimitiveComponent Object Reference") (OtherActor :type "Actor Object Reference") (OtherComp :type "PrimitiveComponent Object Reference") (NormalImpulse :type "Vector Structure") (Hit :type "HitResult Structure (by ref)"))
  (bind _asbp_player (cast `/Game/InfiniteMatrix/Blueprints/BP_Player` OtherActor))
  (bind _returnvalue (- (`/Game/InfiniteMatrix/Blueprints/BP_Player.Health` _asbp_player) 10.0))
  (bind _output_get (set `/Game/InfiniteMatrix/Blueprints/BP_Player.Health` _returnvalue _asbp_player))
  (`/Game/InfiniteMatrix/Blueprints/WB_HealthBar.UpdateHaelthBar` (`/Game/InfiniteMatrix/Blueprints/BP_Player.WB_HealthBar` _asbp_player) _output_get)
  (bind _outactors (`GameplayStatics.GetAllActorsOfClass` "/Game/InfiniteMatrix/Blueprints/BP_Tunnel.BP_Tunnel_C"))
  (`/Game/InfiniteMatrix/Blueprints/BP_Tunnel.UpdateWallColorByHealthValue` (`|GetArrayItem` _outactors) _output_get)
  (if (<= _returnvalue 0.0)
    (`/Game/InfiniteMatrix/Blueprints/BP_Player.DisplayRestart` _asbp_player)
    (set `/Game/InfiniteMatrix/Blueprints/BP_Player.IsDead` true _asbp_player))
  (`self.K2_DestroyActor`))

(fn `UserConstructionScript`)