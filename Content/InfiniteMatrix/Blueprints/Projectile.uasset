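; Projectile actor that flies along the X axis at BulletSpeed and destroys enemies it hits.
; Tick applies the world offset scaled by delta time, while capsule overlaps ignore the player and components tagged "trigger".
; An enemy hit destroys the enemy and, if PlayerRef is valid, increments the player's score, updates its score widget and destroys the projectile.
; Any other hit destroys the projectile directly.
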(event `self.ReceiveTick`
  (params (DeltaSeconds :type "Float (single-precision)"))
  (`self.K2_AddActorWorldOffset` (`KismetMathLibrary.MakeVector` (* DeltaSeconds (`self.BulletSpeed`)))))

(event `self.Capsule.OnComponentBeginOverlap`
  (params (OverlappedComponent :type "PrimitiveComponent Object Reference") (OtherActor :type "Actor Object Reference") (OtherComp :type "PrimitiveComponent Object Reference") (OtherBodyIndex :type Integer) (bFromSweep :type Boolean) (SweepResult :type "HitResult Structure (by ref)"))
  (bind _playerref (`self.PlayerRef`))
  (cast `/Game/InfiniteMatrix/Blueprints/BP_Player` OtherActor
    (:`CastFailed`
      (if (not (`ActorComponent.ComponentHasTag` OtherComp "trigger"))
        (bind _asenemy (cast `/Game/InfiniteMatrix/Blueprints/Enemy` OtherActor)
          (:`then`
            (`self.K2_DestroyActor` _asenemy)
            (`/Engine/EditorBlueprintResources/StandardMacros.IsValid` _playerref
              (:`Is Valid`
                (bind _output_get (set `/Game/InfiniteMatrix/Blueprints/BP_Player.Score` (+ (`/Game/InfiniteMatrix/Blueprints/BP_Player.Score` _playerref) 1) _playerref))
                (`/Game/InfiniteMatrix/Blueprints/WB_Score.UpdateScore` (`/Game/InfiniteMatrix/Blueprints/BP_Player.WB_Score` _playerref) _output_get))))
          (:`CastFailed`
            _))
        (`self.K2_DestroyActor`)))))

(fn `UserConstructionScript`)